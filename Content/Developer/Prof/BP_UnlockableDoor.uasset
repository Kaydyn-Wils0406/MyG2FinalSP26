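; Interactable prop, named as an unlockable door, that moves from its placed transform to an end pose when the player presses E.
; The construction script applies PropMesh to both Prop and EndLocation, so the end pose is visible in the editor.
; Overlapping BP_ExamplePlayer1 shows a prompt and enables input.
; E plays a timeline lerping Prop to EndLocation's relative transform, flags ObjectFallen to suppress the prompt, then disables input on completion.
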(event `self.ReceiveBeginPlay`
  ;[0.15 0.04702 0.0939 0.5] To use this blueprint:
  ; 1. Set the Prop Mesh variable.
  ; 2. Set up the Prop in the desired start location.
  ; 3. Set up the EndLocation mesh to the "end location".
  ; 4. Tell the user to "Press E" or similar, to have the mesh move from the start to the end location (and rotation)
  (set `self.StartingTransform` (`SceneComponent.GetRelativeTransform` (`self.Prop`))))

(event `self.ReceiveActorBeginOverlap`
  (params (OtherActor :type "Actor Object Reference"))
  ;[0.15 0.04702 0.0939 0.5] To use this blueprint:
  ; 1. Set the Prop Mesh variable.
  ; 2. Set up the Prop in the desired start location.
  ; 3. Set up the EndLocation mesh to the "end location".
  ; 4. Tell the user to "Press E" or similar, to have the mesh move from the start to the end location (and rotation)
  (bind _asbp_example_player_1 (cast `/Game/FPFlashlightAnims/Demo/Player/FirstPerson/Blueprints/BP_ExamplePlayer1` OtherActor))
  (bind _pressetointeract (`/Game/FPFlashlightAnims/Demo/Player/FirstPerson/Blueprints/BP_ExamplePlayer1.PressEtoInteract` _asbp_example_player_1))
  (`UserWidget.AddToViewport` _pressetointeract 0)
  (`self.EnableInput` (`GameplayStatics.GetPlayerController` 0))
  (if (`self.bObjectFallen`)
    (`Widget.RemoveFromParent` _pressetointeract)))

(event `self.Sphere.OnComponentEndOverlap`
  (params (OverlappedComponent :type "PrimitiveComponent Object Reference") (OtherActor :type "Actor Object Reference") (OtherComp :type "PrimitiveComponent Object Reference") (OtherBodyIndex :type Integer))
  ;[0.15 0.04702 0.0939 0.5] To use this blueprint:
  ; 1. Set the Prop Mesh variable.
  ; 2. Set up the Prop in the desired start location.
  ; 3. Set up the EndLocation mesh to the "end location".
  ; 4. Tell the user to "Press E" or similar, to have the mesh move from the start to the end location (and rotation)
  (bind _asbp_example_player_1 (cast `/Game/FPFlashlightAnims/Demo/Player/FirstPerson/Blueprints/BP_ExamplePlayer1` OtherActor))
  (`Widget.RemoveFromParent` (`/Game/FPFlashlightAnims/Demo/Player/FirstPerson/Blueprints/BP_ExamplePlayer1.PressEtoInteract` _asbp_example_player_1)))

(event `Key|E`
  (params (Key :type "Key Structure"))
  ;[0.15 0.04702 0.0939 0.5] To use this blueprint:
  ; 1. Set the Prop Mesh variable.
  ; 2. Set up the Prop in the desired start location.
  ; 3. Set up the EndLocation mesh to the "end location".
  ; 4. Tell the user to "Press E" or similar, to have the mesh move from the start to the end location (and rotation)
  (:`Pressed`
    (if true
      (`self.Fall`))))

(event `Fall`
  ;[0.15 0.04702 0.0939 0.5] To use this blueprint:
  ; 1. Set the Prop Mesh variable.
  ; 2. Set up the Prop in the desired start location.
  ; 3. Set up the EndLocation mesh to the "end location".
  ; 4. Tell the user to "Press E" or similar, to have the mesh move from the start to the end location (and rotation)
  (bind (_direction _newtrack_0) (`Timeline|Timeline`)
    (:`Update`
      (`SceneComponent.K2_SetRelativeTransform` (`self.Prop`) (`KismetMathLibrary.TLerp` (`self.StartingTransform`) (`SceneComponent.GetRelativeTransform` (`self.EndLocation`)) _newtrack_0) false false)
      (set `self.bObjectFallen` true))
    (:`Finished`
      (`self.DisableInput` (`GameplayStatics.GetPlayerController` 0)))))

(event `self.Sphere.OnComponentBeginOverlap`
  (params (OverlappedComponent :type "PrimitiveComponent Object Reference") (OtherActor :type "Actor Object Reference") (OtherComp :type "PrimitiveComponent Object Reference") (OtherBodyIndex :type Integer) (bFromSweep :type Boolean) (SweepResult :type "HitResult Structure (by ref)")))

(event `self.Prop.OnComponentBeginOverlap`
  (params (OverlappedComponent :type "PrimitiveComponent Object Reference") (OtherActor :type "Actor Object Reference") (OtherComp :type "PrimitiveComponent Object Reference") (OtherBodyIndex :type Integer) (bFromSweep :type Boolean) (SweepResult :type "HitResult Structure (by ref)")))

(fn `UserConstructionScript`
  (bind _prop_mesh (`self.Prop Mesh`))
  (`StaticMeshComponent.SetStaticMesh` (`self.EndLocation`) _prop_mesh) ; Update the meshes to match the\ndesired Prop Mesh
  (`StaticMeshComponent.SetStaticMesh` (`self.Prop`) _prop_mesh))