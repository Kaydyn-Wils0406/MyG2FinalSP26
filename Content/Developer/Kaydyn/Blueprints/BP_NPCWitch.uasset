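; BP_NPCWitch is a witch NPC that runs a voiced dialogue with the player from the DT_Dialogue data table.
; Entering its sphere registers it on BP_ExamplePlayer1 and shows W_NPCDialogue.
; Each NextLine call shows and plays the next row, aligning and randomly tilting text by speaker.
; An empty row, the table's end or leaving the sphere removes the widget and resets to the start index.
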(event `self.ReceiveBeginPlay`
  (bind _returnvalue (`|CreateWidget` "/Game/Developer/Kaydyn/Blueprints/Widgets/W_NPCDialogue.W_NPCDialogue_C"))
  (set `self.NPCWidget` _returnvalue)
  (set `self.LineIndex` (`self.IndexStart`)))

(event `self.Sphere.OnComponentBeginOverlap`
  (params (OverlappedComponent :type "PrimitiveComponent Object Reference") (OtherActor :type "Actor Object Reference") (OtherComp :type "PrimitiveComponent Object Reference") (OtherBodyIndex :type Integer) (bFromSweep :type Boolean) (SweepResult :type "HitResult Structure (by ref)"))
  (bind _asbp_example_player_1 (cast `/Game/FPFlashlightAnims/Demo/Player/FirstPerson/Blueprints/BP_ExamplePlayer1` OtherActor))
  (bind _output_get (set `self.Player` _asbp_example_player_1))
  (set `/Game/FPFlashlightAnims/Demo/Player/FirstPerson/Blueprints/BP_ExamplePlayer1.NPCWitch` self _output_get)
  (`KismetSystemLibrary.PrintText` "Hello")
  (`UserWidget.AddToViewport` (`self.NPCWidget`) 0))

(event `NextLine`
  (bind _lineindex (`self.LineIndex`))
  (bind _audio (`self.Audio`))
  (bind _textblock_0 (`/Game/Developer/Kaydyn/Blueprints/Widgets/W_NPCDialogue.TextBlock_0` (`self.NPCWidget`)))
  (bind _outrownames (`DataTableFunctionLibrary.GetDataTableRowNames` "/Game/Developer/Kaydyn/Blueprints/DT_Dialogue.DT_Dialogue"))
  (if (> _lineindex (`KismetArrayLibrary.Array_LastIndex` _outrownames))
    (`self.EndDialogue`)
    (else
      (bind _returnvalue (`|GetDataTableRow` "/Game/Developer/Kaydyn/Blueprints/DT_Dialogue.DT_Dialogue" (`|GetArrayItem` _outrownames _lineindex))
        (:`then`
          (if (`KismetTextLibrary.EqualEqual_TextText` (break `/Game/Developer/Kaydyn/Blueprints/S_KaydynStructure` _returnvalue) "")
            (`self.EndDialogue`)
            (else
              (`TextBlock.SetText` (`/Game/Developer/Kaydyn/Blueprints/Widgets/W_NPCDialogue.TextBlock_0` (`self.NPCWidget`)) (break `/Game/Developer/Kaydyn/Blueprints/S_KaydynStructure` _returnvalue))
              (`/Engine/EditorBlueprintResources/StandardMacros.IncrementInt` (`self.LineIndex`)
                (:`  `
                  (`AudioComponent.SetSound` _audio (`.VoicedDialogue_8_B3C5D6B34FBE7DB5B6DCE8B35CEA15D4` (break `/Game/Developer/Kaydyn/Blueprints/S_KaydynStructure` _returnvalue)))
                  (`AudioComponent.Play` _audio 0.0)
                  (switch `/Game/Developer/Kaydyn/Blueprints/E_Speaker` (`.SpeakerStructure_7_31B056F74D6A388BB4FAFC808B51457F` (break `/Game/Developer/Kaydyn/Blueprints/S_KaydynStructure` _returnvalue))
                    (:`NewEnumerator0`
                      (`Widget.SetRenderTransformAngle` _textblock_0 (`KismetMathLibrary.RandomFloatInRange` -2.0 -1.0))
                      (set `TextLayoutWidget.Justification` "Left" _textblock_0))
                    (:`NewEnumerator1`
                      (`Widget.SetRenderTransformAngle` _textblock_0 (`KismetMathLibrary.RandomFloatInRange` 1.0 2.0))
                      (set `TextLayoutWidget.Justification` "Right" _textblock_0))))))))))))

(event `EndDialogue`
  (`Widget.RemoveFromParent` (`self.NPCWidget`))
  (set `self.LineIndex` (`self.IndexStart`))
  (set `/Game/FPFlashlightAnims/Demo/Player/FirstPerson/Blueprints/BP_ExamplePlayer1.NPCWitch` null (`self.Player`))
  (set `self.Player` null))

(event `self.Sphere.OnComponentEndOverlap`
  (params (OverlappedComponent :type "PrimitiveComponent Object Reference") (OtherActor :type "Actor Object Reference") (OtherComp :type "PrimitiveComponent Object Reference") (OtherBodyIndex :type Integer))
  (cast `/Game/FPFlashlightAnims/Demo/Player/FirstPerson/Blueprints/BP_ExamplePlayer1` OtherActor)
  (`self.EndDialogue`))

(fn `UserConstructionScript`
  (`parent.UserConstructionScript`))