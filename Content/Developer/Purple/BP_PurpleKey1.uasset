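; BP_PurpleKey1 is a purple key pickup that the player collects by walking into its box.
; On overlap with BP_ExamplePlayer1, it sets that player's ObtainedPurpleKey1 flag, increments Keycount and prints the new total.
; It then destroys itself and calls ShowKeyWidget on player character 0, fetched separately from the overlapping actor.
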(event `self.Box.OnComponentBeginOverlap`
  (params (OverlappedComponent :type "PrimitiveComponent Object Reference") (OtherActor :type "Actor Object Reference") (OtherComp :type "PrimitiveComponent Object Reference") (OtherBodyIndex :type Integer) (bFromSweep :type Boolean) (SweepResult :type "HitResult Structure (by ref)"))
  (bind _asbp_example_player_1 (cast `/Game/FPFlashlightAnims/Demo/Player/FirstPerson/Blueprints/BP_ExamplePlayer1` OtherActor))
  (set `/Game/FPFlashlightAnims/Demo/Player/FirstPerson/Blueprints/BP_ExamplePlayer1.ObtainedPurpleKey1` true _asbp_example_player_1)
  (bind _keycount (`/Game/FPFlashlightAnims/Demo/Player/FirstPerson/Blueprints/BP_ExamplePlayer1.keycount` _asbp_example_player_1))
  (set `/Game/FPFlashlightAnims/Demo/Player/FirstPerson/Blueprints/BP_ExamplePlayer1.keycount` (+ _keycount 1) _asbp_example_player_1)
  (`KismetSystemLibrary.PrintString` (`KismetStringLibrary.Concat_StrStr` "The Player has " (`KismetStringLibrary.Conv_IntToString` _keycount) " key(s)."))
  (`|ExecutionSequence`
    (:`then_0`
      (`self.K2_DestroyActor`))
    (:`then_1`
      (bind _asbp_example_player_1_2 (cast `/Game/FPFlashlightAnims/Demo/Player/FirstPerson/Blueprints/BP_ExamplePlayer1` (`GameplayStatics.GetPlayerCharacter` 0)))
      (`/Game/FPFlashlightAnims/Demo/Player/FirstPerson/Blueprints/BP_ExamplePlayer1.ShowKeyWidget` _asbp_example_player_1_2))))

(fn `UserConstructionScript`)