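; BP_LevelConnectionPtoK is a level-exit trigger that sends the player from the Purple area to L_Kaydyn once all three purple keys are collected.
; On Box overlap it casts to BP_ExamplePlayer1, checks the three key flags in nested branches, and opens the level by object reference if all pass.
; Any missing key briefly shows the player's WMissingKey widget before removing it.
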(event `self.Box.OnComponentBeginOverlap`
  (params (OverlappedComponent :type "PrimitiveComponent Object Reference") (OtherActor :type "Actor Object Reference") (OtherComp :type "PrimitiveComponent Object Reference") (OtherBodyIndex :type Integer) (bFromSweep :type Boolean) (SweepResult :type "HitResult Structure (by ref)"))
  (bind _asbp_example_player_1 (cast `/Game/FPFlashlightAnims/Demo/Player/FirstPerson/Blueprints/BP_ExamplePlayer1` OtherActor))
  (if (`/Game/FPFlashlightAnims/Demo/Player/FirstPerson/Blueprints/BP_ExamplePlayer1.ObtainedPurpleKey1` _asbp_example_player_1)
    (if (`/Game/FPFlashlightAnims/Demo/Player/FirstPerson/Blueprints/BP_ExamplePlayer1.ObtainedPurpleKey2` _asbp_example_player_1)
      (if (`/Game/FPFlashlightAnims/Demo/Player/FirstPerson/Blueprints/BP_ExamplePlayer1.ObtainedPurpleKey3` _asbp_example_player_1)
        (`KismetSystemLibrary.PrintString` "Player has hit the box")
        (`GameplayStatics.OpenLevelBySoftObjectPtr` "/Game/Developer/Kaydyn/L_Kaydyn.L_Kaydyn")
        (else
          (bind _w_missingkey (`/Game/FPFlashlightAnims/Demo/Player/FirstPerson/Blueprints/BP_ExamplePlayer1.W_MissingKey` _asbp_example_player_1))
          (`UserWidget.AddToViewport` _w_missingkey 0)
          (`KismetSystemLibrary.Delay` 3.0)
          (`Widget.RemoveFromParent` _w_missingkey)))
      (else
        (bind _w_missingkey_2 (`/Game/FPFlashlightAnims/Demo/Player/FirstPerson/Blueprints/BP_ExamplePlayer1.W_MissingKey` _asbp_example_player_1))
        (`UserWidget.AddToViewport` _w_missingkey_2 0)
        (`KismetSystemLibrary.Delay` 3.0)
        (`Widget.RemoveFromParent` _w_missingkey_2)))
    (else
      (bind _w_missingkey_3 (`/Game/FPFlashlightAnims/Demo/Player/FirstPerson/Blueprints/BP_ExamplePlayer1.W_MissingKey` _asbp_example_player_1))
      (`UserWidget.AddToViewport` _w_missingkey_3 0)
      (`KismetSystemLibrary.Delay` 3.0)
      (`Widget.RemoveFromParent` _w_missingkey_3))))

(fn `UserConstructionScript`)